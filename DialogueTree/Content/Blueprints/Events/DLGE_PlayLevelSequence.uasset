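; Dialogue graph event that plays a chosen Cinematic level sequence, blocking the dialogue until it finishes.
; On play, it spawns a LevelSequenceActor, with PlayFromSpeakerLocation toggling a transform-origin override.
; It binds the main and additional speakers' actors by using their dialogue names as binding tags.
; Skipping jumps the sequence to its end, and the finish callback releases blocking and destroys the spawned actor.
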(event `self.OnPlayEvent`
  (params (InSpeaker :type "SpeakerActorEntry Structure") (OtherSpeakers :type "Array of SpeakerActorEntry Structure (by ref)"))
  ;[1 1 1] Start Blocking
  (`self.StartBlocking`)
  ;[1 1 1] Create the sequence actor
  (bind _newparam (`self.SpawnLevelSequence` (`.Actor` (break `SpeakerActorEntry` InSpeaker))))
  (bind _output_get (set `self.LevelSequenceActor` _newparam))
  (`/Engine/EditorBlueprintResources/StandardMacros.IsValid` _output_get
    (:`Is Valid`
      ;[1 1 1] Bind Speakers Into Sequence As Necessary
      (`self.BindSpeaker` InSpeaker (`self.LevelSequenceActor`))
      (`self.BindAdditionalSpeakers` OtherSpeakers (`self.LevelSequenceActor`))
      (add `MovieSceneSequencePlayer.OnFinished` (`LevelSequenceActor.SequencePlayer` (`self.LevelSequenceActor`)) (delegate `OnFinished_Event`))
      ;[1 1 1] Start playing
      (`MovieSceneSequencePlayer.Play` (`LevelSequenceActor.SequencePlayer` (`self.LevelSequenceActor`))))))

(event `OnFinished_Event`
  ;[1 1 1] When the cinematic is done, stop blocking and destroy the spawned sequence
  (`self.StopBlocking`)
  (`Actor.K2_DestroyActor` (`self.LevelSequenceActor`)))

(event `self.OnSkipped`
  (bind _levelsequenceactor (`self.LevelSequenceActor`))
  (`/Engine/EditorBlueprintResources/StandardMacros.IsValid` _levelsequenceactor
    (:`Is Valid`
      (`MovieSceneSequencePlayer.GoToEndAndStop` (`LevelSequenceActor.SequencePlayer` _levelsequenceactor)))))

(fn `BindAdditionalSpeakers`
  (params (AdditionalSpeakers :type "Array of SpeakerActorEntry Structure") (InSequence :type "LevelSequenceActor Object Reference"))
  (for _array_element AdditionalSpeakers
    (`self.BindSpeaker` _array_element InSequence)))

(fn `BindSpeaker`
  (params (InSpeaker :type "SpeakerActorEntry Structure") (InSequence :type "LevelSequenceActor Object Reference"))
  (bind (_actor _speakercomponent) (break `SpeakerActorEntry` InSpeaker))
  (`LevelSequenceActor.AddBindingByTag` (`local.InSequence`) (`DialogueSpeakerComponent.GetDialogueName` _speakercomponent) _actor false))

(fn `GetGraphDescription`
  (returns (ReturnValue :type Text))
  (return (`|FormatText` "Play Cinematic \"{Cinematic}\"" (`KismetSystemLibrary.GetDisplayName` (`self.Cinematic`)))))

(fn `IsValidEvent`
  (returns (ReturnValue :type Boolean))
  (`/Engine/EditorBlueprintResources/StandardMacros.IsValid` (`self.Cinematic`)
    (:`Is Valid`
      (return true))
    (:`Is Not Valid`
      (return false))))

(fn `SpawnLevelSequence`
  (params (SpeakerActor :type "Actor Object Reference"))
  (returns (NewParam :type "LevelSequenceActor Object Reference"))
  (locals (SpawnLocation :type "Vector Structure") (SpawnRotation :type "Rotator Structure") (SpawnedSequence :type "LevelSequenceActor Object Reference"))
  (bind _spawnedsequence (`local.SpawnedSequence`))
  ;[1 1 1] Spawn at the actor's location
  (set `local.SpawnLocation` (`Actor.K2_GetActorLocation` SpeakerActor))
  (set `local.SpawnRotation` (`Actor.K2_GetActorRotation` SpeakerActor))
  (bind _returnvalue (`self.SpawnActorToCurrentWorld` "/Script/LevelSequence.LevelSequenceActor" (0.0 0.0 0.0) (struct) null))
  (bind _aslevel_sequence_actor (cast `LevelSequenceActor` _returnvalue))
  (bind _output_get (set `local.SpawnedSequence` _aslevel_sequence_actor))
  ;[1 1 1] Set the actual sequence to play
  (`LevelSequenceActor.SetSequence` _output_get (`self.Cinematic`))
  ;[1 1 1] Set relative vs absolute location
  (set `LevelSequenceActor.bOverrideInstanceData` (`self.PlayFromSpeakerLocation`) _spawnedsequence)
  (bind _asdefault_level_sequence_instance_data (cast `DefaultLevelSequenceInstanceData` (`LevelSequenceActor.DefaultInstanceData` _spawnedsequence)))
  (set `DefaultLevelSequenceInstanceData.TransformOrigin` (`Actor.GetTransform` (`local.SpawnedSequence`)) _asdefault_level_sequence_instance_data)
  (return (`local.SpawnedSequence`)))